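; PickUpGem is a collectible gem that raises the coin count when the player touches it.
; Overlapping its Sphere with BP_Player plays a collect sound, calls IncreaseCurrentCoins on BP_GameMode and destroys the actor.
; A separate PowerUpCollision overlap checks the player's MagnetOn flag and quickly eases the Sphere toward the player's location, passing that world position as a relative target.
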(event `self.Sphere.OnComponentBeginOverlap`
  (params (OverlappedComponent :type "PrimitiveComponent Object Reference") (OtherActor :type "Actor Object Reference") (OtherComp :type "PrimitiveComponent Object Reference") (OtherBodyIndex :type Integer) (bFromSweep :type Boolean) (SweepResult :type "HitResult Structure (by ref)"))
  (cast `/Game/Blueprints/BP_Player` OtherActor)
  (`GameplayStatics.PlaySoundAtLocation` "/Game/Assets/Audio/A_CoinCollect.A_CoinCollect" (`self.K2_GetActorLocation`) (struct) 1.0 1.0 0.0 null null null)
  (bind _asbp_game_mode (cast `/Game/Blueprints/BP_GameMode` (`GameplayStatics.GetGameMode`)))
  (`/Game/Blueprints/BP_GameMode.IncreaseCurrentCoins` _asbp_game_mode)
  (`self.K2_DestroyActor`))

(event `self.PowerUpCollision.OnComponentBeginOverlap`
  (params (OverlappedComponent :type "PrimitiveComponent Object Reference") (OtherActor :type "Actor Object Reference") (OtherComp :type "PrimitiveComponent Object Reference") (OtherBodyIndex :type Integer) (bFromSweep :type Boolean) (SweepResult :type "HitResult Structure (by ref)"))
  (bind _asbp_player (cast `/Game/Blueprints/BP_Player` OtherActor))
  (if (`/Game/Blueprints/BP_Player.MagnetOn?` _asbp_player)
    (`KismetSystemLibrary.MoveComponentTo` (`self.Sphere`) (`self.K2_GetActorLocation` _asbp_player) (struct) false true 0.05 true)))

(fn `UserConstructionScript`)