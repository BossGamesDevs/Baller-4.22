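; BP_Projectile is a hazard actor that ends the player's run when its static mesh hits the player pawn.
; On that hit it plays a shock sound, has BP_Player save its distance to the game instance, then after a short delay zeroes BP_GameMode's coins and calls GameComplete on the player.
; A hit on anything else destroys the projectile after a delay; no movement logic is scripted here.
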(event `self.StaticMesh.OnComponentHit`
  (params (HitComponent :type "PrimitiveComponent Object Reference") (OtherActor :type "Actor Object Reference") (OtherComp :type "PrimitiveComponent Object Reference") (NormalImpulse :type "Vector Structure") (Hit :type "HitResult Structure (by ref)"))
  (if (== OtherActor (`GameplayStatics.GetPlayerPawn` 0))
    (bind _asbp_player (cast `/Game/Blueprints/BP_Player` OtherActor))
    (`GameplayStatics.PlaySoundAtLocation` "/Game/Assets/Audio/A_Shock.A_Shock" (`SceneComponent.K2_GetComponentLocation` (`/Game/Blueprints/BP_Player.Player` _asbp_player)))
    (`/Game/Blueprints/BP_Player.SaveDistanceToGameInstance` _asbp_player)
    (`KismetSystemLibrary.Delay` 0.5)
    (bind _asbp_game_mode (cast `/Game/Blueprints/BP_GameMode` (`GameplayStatics.GetGameMode`)))
    (set `/Game/Blueprints/BP_GameMode.CurrentCoins` 0 _asbp_game_mode)
    (`/Game/Blueprints/BP_Player.GameComplete` _asbp_player)
    (else
      (`KismetSystemLibrary.Delay` 2.0)
      (`self.K2_DestroyActor`))))

(fn `UserConstructionScript`)