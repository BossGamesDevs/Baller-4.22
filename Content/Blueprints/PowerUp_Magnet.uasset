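; A magnet power-up pickup that grants the player the magnet ability.
; On BeginPlay it caches the BP_Player reference; when the player pawn overlaps its sphere, it plays a sound, calls PowerUpMagnet on the player and destroys itself.
; Spin and brief slow-motion logic exist in the graph but are disconnected and never run.
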(event `self.ReceiveBeginPlay`
  (bind _asbp_player (cast `/Game/Blueprints/BP_Player` (`GameplayStatics.GetPlayerPawn` 0)))
  (set `self.BP_Player` _asbp_player))

(event `self.ReceiveTick`
  (params (DeltaSeconds :type "Float (single-precision)")))

(event `self.Sphere.OnComponentBeginOverlap`
  (params (OverlappedComponent :type "PrimitiveComponent Object Reference") (OtherActor :type "Actor Object Reference") (OtherComp :type "PrimitiveComponent Object Reference") (OtherBodyIndex :type Integer) (bFromSweep :type Boolean) (SweepResult :type "HitResult Structure (by ref)"))
  (if (== OtherActor (`GameplayStatics.GetPlayerPawn` 0))
    (`GameplayStatics.PlaySoundAtLocation` "/Game/Assets/Audio/Enter_Simulate.Enter_Simulate" (`self.K2_GetActorLocation`) (struct) 1.0 1.0 0.0 null null null)
    (`/Game/Blueprints/BP_Player.PowerUp_Magnet` (`self.BP_Player`))
    (`self.K2_DestroyActor`)))

(fn `UserConstructionScript`)