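; PickUpChar is a coin pickup that raises the score when something overlaps its capsule.
; It caches the player pawn on BeginPlay and spins the Coin component each tick by a fixed, frame-rate-dependent step.
; Any overlap, with no check on the other actor, plays a collect sound at the player, updates score and top score through BP_GameMode, then destroys the pickup.
; A brief slow-motion effect is left unconnected.
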(event `self.ReceiveBeginPlay`
  (bind _asbp_player (cast `/Game/Blueprints/BP_Player` (`GameplayStatics.GetPlayerPawn` 0)))
  (set `self.BP_Player` _asbp_player))

(event `self.ReceiveTick`
  (params (DeltaSeconds :type "Float (single-precision)"))
  (`SceneComponent.K2_AddRelativeRotation` (`self.Coin`) (struct :`Yaw` 5.0) false false))

(event `self.CapsuleComponent.OnComponentBeginOverlap`
  (params (OverlappedComponent :type "PrimitiveComponent Object Reference") (OtherActor :type "Actor Object Reference") (OtherComp :type "PrimitiveComponent Object Reference") (OtherBodyIndex :type Integer) (bFromSweep :type Boolean) (SweepResult :type "HitResult Structure (by ref)"))
  (`GameplayStatics.PlaySoundAtLocation` "/Game/Assets/Audio/A_CoinCollect.A_CoinCollect" (`self.K2_GetActorLocation` (`self.BP_Player`)))
  (bind _asbp_game_mode (cast `/Game/Blueprints/BP_GameMode` (`GameplayStatics.GetGameMode`)))
  (`/Game/Blueprints/BP_GameMode.IncreaseScore` _asbp_game_mode)
  (`/Game/Blueprints/BP_GameMode.UpdateTopScore` _asbp_game_mode)
  (`self.K2_DestroyActor`))

(fn `UserConstructionScript`)