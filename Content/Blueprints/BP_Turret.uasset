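; BP_Turret is an enemy turret that tracks the player and fires projectiles when they come within attack range.
; Tick updates the range flag and smoothly rotates the barrel toward a point offset along world X from the player, a fixed lead.
; A self-calling delay loop started at BeginPlay spawns BP_Projectile at the barrel socket with a shot sound, polls while out of range, and ends once the player's game has ended.
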(event `self.ReceiveBeginPlay`
  ;[1 1 1] Begin Play
  (bind _asbp_player (cast `/Game/Blueprints/BP_Player` (`GameplayStatics.GetPlayerPawn` 0)))
  (set `self.BP_Player` _asbp_player)
  (bind _asbp_game_mode (cast `/Game/Blueprints/BP_GameMode` (`GameplayStatics.GetGameMode`)))
  (set `self.BP_GameMode` _asbp_game_mode)
  (`self.ShootAtPlayer`))

(event `self.ReceiveTick`
  (params (DeltaSeconds :type "Float (single-precision)"))
  ;[1 1 1] TICK
  (set `self.DeltaTime` DeltaSeconds)
  (`self.RangeCheck`)
  (`self.TurretRoation`))

(event `TurretRoation`
  (bind _turret_barrel (`self.Turret_Barrel`))
  (bind (_returnvalue_x _returnvalue_y _returnvalue_z) (`KismetMathLibrary.BreakVector` (`SceneComponent.K2_GetComponentLocation` (`/Game/Blueprints/BP_Player.Player` (`self.BP_Player`)))))
  ;[1 1 1] Turret Rotation
  (if true
    (if (`self.InRange`)
      (`SceneComponent.K2_SetWorldRotation` _turret_barrel (`KismetMathLibrary.RInterpTo` (`SceneComponent.K2_GetComponentRotation` _turret_barrel) (`KismetMathLibrary.MakeRotator` 0.0 (.pitch (`KismetMathLibrary.FindLookAtRotation` (`SceneComponent.K2_GetComponentLocation` (`self.Turret_Barrel`)) (`KismetMathLibrary.MakeVector` (+ _returnvalue_x 500.0) _returnvalue_y _returnvalue_z))) (.yaw (`KismetMathLibrary.FindLookAtRotation` (`SceneComponent.K2_GetComponentLocation` (`self.Turret_Barrel`)) (`KismetMathLibrary.MakeVector` (+ _returnvalue_x 500.0) _returnvalue_y _returnvalue_z)))) (`self.DeltaTime`) (`self.RotationSpeed`)) false false)
      (set `self.HasAim?` true))))

(event `RangeCheck`
  ;[1 1 1] Range Check
  (if true
    (if (< (`self.GetDistanceTo` self (`GameplayStatics.GetPlayerPawn` 0)) (`self.AttackRange`))
      (set `self.InRange` true)
      (else
        (set `self.InRange` false)))))

(event `ShootAtPlayer`
  ;[1 1 1] Shoot Player
  (if (not (`/Game/Blueprints/BP_Player.bGameEnded` (`self.BP_Player`)))
    (if (`self.InRange`)
      (`KismetSystemLibrary.RetriggerableDelay` 0.15)
      (`|SpawnActorFromClass` "/Game/Blueprints/BP_Projectile.BP_Projectile_C" (`SceneComponent.GetSocketTransform` (`self.Turret_Barrel`) "Sock_Barrel" "RTS_World") "Undefined" "OverrideRootScale" null null)
      (`GameplayStatics.PlaySoundAtLocation` "/Game/Assets/Audio/A_TurretShot.A_TurretShot" (`SceneComponent.K2_GetComponentLocation` (`self.Turret_Barrel`)) (struct) 1.0 1.0 0.0 null null null)
      (`KismetSystemLibrary.RetriggerableDelay` (`self.FireRate`))
      (`self.ShootAtPlayer`)
      (else
        (`KismetSystemLibrary.RetriggerableDelay` 0.5)
        (`self.ShootAtPlayer`)))))

(fn `UserConstructionScript`)