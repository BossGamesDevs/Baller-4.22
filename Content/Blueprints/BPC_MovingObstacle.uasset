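; Moving obstacle actor that endlessly sways its Obstacle component back and forth along the relative Y axis.
; BeginPlay chains two eased MoveComponentTo calls in a loop, both timed by SwaySpeed, which acts as a duration.
; Each move offsets from the component's current location, so it travels between its start and a point on +Y.
; Overlap and Tick events are unused.
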(event `self.ReceiveBeginPlay`
  (bind (_relativelocation_x _relativelocation_y _relativelocation_z) (`KismetMathLibrary.BreakVector` (`SceneComponent.RelativeLocation` (`self.Obstacle`))))
  (bind (_relativelocation_x_2 _relativelocation_y_2 _relativelocation_z_2) (`KismetMathLibrary.BreakVector` (`SceneComponent.RelativeLocation` (`self.Obstacle`))))
  (`parent.ReceiveBeginPlay`)
  (`KismetSystemLibrary.MoveComponentTo` (`self.Obstacle`) (`KismetMathLibrary.MakeVector` _relativelocation_x_2 (+ _relativelocation_y_2 1000.0) _relativelocation_z_2) (struct) true true (`self.SwaySpeed`) :!label _label)
  (`KismetSystemLibrary.MoveComponentTo` (`self.Obstacle`) (`KismetMathLibrary.MakeVector` _relativelocation_x (+ _relativelocation_y -1000.0) _relativelocation_z) (struct) true true (`self.SwaySpeed`))
  (goto _label))

(fn `UserConstructionScript`
  (`parent.UserConstructionScript`))