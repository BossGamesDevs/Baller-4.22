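; A coin-banking pickup that banks the player's coins when they overlap its sphere, then destroys itself.
; On overlap by BP_Player it shows banked-coins text on BP_HUD, plays a collection sound, calls BP_GameMode to update the hard wallet and bank points, and flashes the cached player yellow.
; Unconnected leftover nodes for sphere rotation and a brief slow-motion effect never run.
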(event `self.ReceiveBeginPlay`
  (bind _asbp_player (cast `/Game/Blueprints/BP_Player` (`GameplayStatics.GetPlayerPawn` 0)))
  (set `self.BP_Player` _asbp_player))

(event `self.ReceiveTick`
  (params (DeltaSeconds :type "Float (single-precision)")))

(event `self.Sphere.OnComponentBeginOverlap`
  (params (OverlappedComponent :type "PrimitiveComponent Object Reference") (OtherActor :type "Actor Object Reference") (OtherComp :type "PrimitiveComponent Object Reference") (OtherBodyIndex :type Integer) (bFromSweep :type Boolean) (SweepResult :type "HitResult Structure (by ref)"))
  (cast `/Game/Blueprints/BP_Player` OtherActor)
  (bind _asbp_hud (cast `/Game/Blueprints/BP_HUD` (`PlayerController.GetHUD` (`GameplayStatics.GetPlayerController` 0))))
  (`/Game/Blueprints/BP_HUD.ShowBankedCoinsText` _asbp_hud)
  (`GameplayStatics.PlaySoundAtLocation` "/Game/Assets/Audio/BankCollected_Cue.BankCollected_Cue" (`self.K2_GetActorLocation`))
  (bind _asbp_game_mode (cast `/Game/Blueprints/BP_GameMode` (`GameplayStatics.GetGameMode`)))
  (`/Game/Blueprints/BP_GameMode.UpdateHardWallet` _asbp_game_mode)
  (`/Game/Blueprints/BP_GameMode.BankPoints` _asbp_game_mode)
  (`/Game/Blueprints/BP_Player.FlashColour_Yellow` (`self.BP_Player`))
  (`self.K2_DestroyActor`))

(fn `UserConstructionScript`)