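; A collectible gem pickup that plays a sound, increments the game mode's gem count and destroys itself when the player overlaps its Sphere.
; A separate PowerUpCollision overlap starts a timeline that interpolates the pickup toward the player, adding a track offset, while the player's magnet is on.
; The timeline stops when the magnet is off.
; Rotation and slow-motion nodes are present but unconnected.
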(event `self.ReceiveBeginPlay`
  (bind _asbp_player (cast `/Game/Blueprints/BP_Player` (`GameplayStatics.GetPlayerPawn` 0)))
  (set `self.BP_Player` _asbp_player))

(event `self.ReceiveTick`
  (params (DeltaSeconds :type "Float (single-precision)")))

(event `self.Sphere.OnComponentBeginOverlap`
  (params (OverlappedComponent :type "PrimitiveComponent Object Reference") (OtherActor :type "Actor Object Reference") (OtherComp :type "PrimitiveComponent Object Reference") (OtherBodyIndex :type Integer) (bFromSweep :type Boolean) (SweepResult :type "HitResult Structure (by ref)"))
  (if (== OtherActor (`GameplayStatics.GetPlayerPawn` 0))
    (`GameplayStatics.PlaySoundAtLocation` "/Game/Assets/Audio/A_CoinCollect.A_CoinCollect" (`self.K2_GetActorLocation`))
    (bind _asbp_game_mode (cast `/Game/Blueprints/BP_GameMode` (`GameplayStatics.GetGameMode`)))
    (`/Game/Blueprints/BP_GameMode.IncreaseCurrentGems` _asbp_game_mode)
    (`self.K2_DestroyActor`)))

(event `self.PowerUpCollision.OnComponentBeginOverlap`
  (params (OverlappedComponent :type "PrimitiveComponent Object Reference") (OtherActor :type "Actor Object Reference") (OtherComp :type "PrimitiveComponent Object Reference") (OtherBodyIndex :type Integer) (bFromSweep :type Boolean) (SweepResult :type "HitResult Structure (by ref)"))
  (bind _returnvalue_location (`KismetMathLibrary.BreakTransform` (`self.GetTransform`)))
  (if (== OtherActor (`GameplayStatics.GetPlayerPawn` 0))
    (bind (_direction _newtrack_0) (`Timeline|ChaseTimeLine` :!via `PlayFromStart` :!label _label)
      (:`Update`
        (if (`/Game/Blueprints/BP_Player.MagnetOn?` (`self.BP_Player`))
          (`self.K2_SetActorLocation` (+ _newtrack_0 (`KismetMathLibrary.VInterpTo` _returnvalue_location (`self.K2_GetActorLocation` (`self.BP_Player`)) (`GameplayStatics.GetWorldDeltaSeconds`) 20.0)))
          (else
            (goto _label :!via `Stop`)))))))

(fn `UserConstructionScript`)