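; Game instance that holds persistent shop state: owned and chosen skins and particle effects, plus banked gems.
; On Init it loads the MySave slot and copies its values into GI variables, or creates and saves a new save object if none exists.
; Shutdown and a callable Save event share one path that writes those variables back to the save object and slot.
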(event `self.ReceiveInit`
  (bind _returnvalue (`GameplayStatics.DoesSaveGameExist` "MySave"))
  (if _returnvalue
    (`KismetSystemLibrary.PrintString` "Mysave Exists")
    (bind _returnvalue_2 (`GameplayStatics.LoadGameFromSlot` "MySave"))
    (bind _asbp_save_game_shop (cast `/Game/MainMenu/BP_SaveGame_SHOP` _returnvalue_2))
    (set `self.SaveGameReference` _asbp_save_game_shop)
    ;[1 0.3944 0.8064] CacheSavedGameVariables
    (`|ExecutionSequence`
      (:`then_0`
        (set `self.GI_bHasSkins` (`/Game/MainMenu/BP_SaveGame_SHOP.SavedbHasSkins` (`self.SaveGameReference`))))
      (:`then_1`
        (set `self.GI_ChosenSkinIndex` (`/Game/MainMenu/BP_SaveGame_SHOP.SavedChosenSkinIndex` (`self.SaveGameReference`))))
      (:`then_2`
        (set `self.GI_BankedGems` (`/Game/MainMenu/BP_SaveGame_SHOP.SavedBankedGems` (`self.SaveGameReference`))))
      (:`then_3`
        (set `self.GI_ParticleSystemNiagara` (`/Game/MainMenu/BP_SaveGame_SHOP.SavedParticleColour` (`self.SaveGameReference`))))
      (:`then_4`
        (set `self.GI_ParticleSystemArray` (`/Game/MainMenu/BP_SaveGame_SHOP.SavedParticleSystemArray` (`self.SaveGameReference`))))
      (:`then_5`
        (set `self.GI_bHasParticles` (`/Game/MainMenu/BP_SaveGame_SHOP.SavedbHasParticles` (`self.SaveGameReference`))))
      (:`then_6`
        (set `self.GI_ChosenParticleIndex` (`/Game/MainMenu/BP_SaveGame_SHOP.SavedChosenParticleIndex` (`self.SaveGameReference`)))))
    (else
      (`KismetSystemLibrary.PrintString` "MySave Created")
      (bind _returnvalue_3 (`GameplayStatics.CreateSaveGameObject` "/Game/MainMenu/BP_SaveGame_SHOP.BP_SaveGame_SHOP_C"))
      (bind _output_get (set `self.SaveGameReference` _returnvalue_3))
      (`GameplayStatics.SaveGameToSlot` _output_get "MySave"))))

(event `self.ReceiveShutdown`
  (bind _savegamereference (`self.SaveGameReference`))
  ;[1 1 1] Cache_GameInstance_Variables[SaveGame on Shutdown]
  (set `/Game/MainMenu/BP_SaveGame_SHOP.SavedChosenSkinIndex` (`self.GI_ChosenSkinIndex`) _savegamereference :!label _label)
  (set `/Game/MainMenu/BP_SaveGame_SHOP.SavedbHasSkins` (`self.GI_bHasSkins`) _savegamereference)
  (set `/Game/MainMenu/BP_SaveGame_SHOP.SavedBankedGems` (`self.GI_BankedGems`) _savegamereference)
  (set `/Game/MainMenu/BP_SaveGame_SHOP.SavedParticleColour` (`self.GI_ParticleSystemNiagara`) _savegamereference)
  (set `/Game/MainMenu/BP_SaveGame_SHOP.SavedParticleSystemArray` (`self.GI_ParticleSystemArray`) _savegamereference)
  (set `/Game/MainMenu/BP_SaveGame_SHOP.SavedbHasParticles` (`self.GI_bHasParticles`) _savegamereference)
  (set `/Game/MainMenu/BP_SaveGame_SHOP.SavedChosenParticleIndex` (`self.GI_ChosenParticleIndex`) _savegamereference)
  (`GameplayStatics.SaveGameToSlot` _savegamereference "MySave")
  (`KismetSystemLibrary.PrintString` "SAVED"))

(event `Save`
  ;[1 1 1] Cache_GameInstance_Variables[SaveGame on Shutdown]
  (goto _label))