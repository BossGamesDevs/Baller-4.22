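; Endless-runner floor tile that populates itself with random content and chains the level onward.
; Construction always adds a gem, a wall at one set tile index, and one random pick of bank coin, magnet, speed boost, index-gated turrets, spin man or tornado.
; BeginPlay animates the spin man by timeline or keeps the tornado wandering.
; KillZone calls the player's GameComplete; EndTrigger requests another tile from BP_GameMode, then destroys this one after a delay.
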(event `self.ReceiveBeginPlay`
  (bind _returnvalue (`KismetMathLibrary.RandomFloatInRange` -500.0 500.0))
  (bind _tornado (`self.Tornado`))
  (bind _spinnyman (`self.SpinnyMan`))
  (bind (_relativelocation_x _relativelocation_y) (`KismetMathLibrary.BreakVector` (`SceneComponent.RelativeLocation` _tornado)))
  (`KismetSystemLibrary.Delay` 0.2)
  (if (`self.bHasSpinManSpawned?`)
    (bind (_direction _spin _location) (`Timeline|Timeline_0` :!via `PlayFromStart`)
      (:`Update`
        (`/Engine/EditorBlueprintResources/StandardMacros.IsValid` (`self.SpinnyMan`)
          (:`Is Valid`
            (`SceneComponent.K2_AddRelativeRotation` _spinnyman (`KismetMathLibrary.MakeRotator` 0.0 0.0 _spin) false false)
            (`SceneComponent.K2_AddRelativeLocation` _spinnyman (`KismetMathLibrary.MakeVector` 0.0 0.0 _location) false false)))))
    (elif (`self.bHasTornadoSpawned?`)
      (set `self.TornadoLocationInit` (`SceneComponent.RelativeLocation` _tornado) :!label _label)
      (set `self.TornadoLocationTarget` (`KismetMathLibrary.MakeVector` (+ _relativelocation_x _returnvalue) (+ _relativelocation_y _returnvalue)))
      (`KismetSystemLibrary.MoveComponentTo` (`self.Tornado`) (`self.TornadoLocationTarget`) (struct) true false 1.0 true)
      (goto _label))))

(event `self.KillZone.OnComponentBeginOverlap`
  (params (OverlappedComponent :type "PrimitiveComponent Object Reference") (OtherActor :type "Actor Object Reference") (OtherComp :type "PrimitiveComponent Object Reference") (OtherBodyIndex :type Integer) (bFromSweep :type Boolean) (SweepResult :type "HitResult Structure (by ref)"))
  (bind _asbp_player (cast `/Game/Blueprints/BP_Player` OtherActor))
  (`/Game/Blueprints/BP_Player.GameComplete` _asbp_player))

(event `self.EndTrigger.OnComponentBeginOverlap`
  (params (OverlappedComponent :type "PrimitiveComponent Object Reference") (OtherActor :type "Actor Object Reference") (OtherComp :type "PrimitiveComponent Object Reference") (OtherBodyIndex :type Integer) (bFromSweep :type Boolean) (SweepResult :type "HitResult Structure (by ref)"))
  (cast `/Game/Blueprints/BP_Player` OtherActor)
  (bind _asbp_game_mode (cast `/Game/Blueprints/BP_GameMode` (`GameplayStatics.GetGameMode`)))
  (`/Game/Blueprints/BP_GameMode.AddFloorTile` _asbp_game_mode)
  (`KismetSystemLibrary.Delay` 3.0)
  (`self.K2_DestroyActor`))

(fn `GetAttachTransform`
  (returns (AttachTransform :type "Transform Structure"))
  (return (`SceneComponent.K2_GetComponentToWorld` (`self.AttachPoint`))))

(fn `GetSpawnPoints`
  (set `self.SpawnPoints` (`|MakeArray` (`SceneComponent.GetRelativeTransform` (`self.SpawnPoint1`)) (`SceneComponent.GetRelativeTransform` (`self.SpawnPoint2`)) (`SceneComponent.GetRelativeTransform` (`self.SpawnPoint3`)) (`SceneComponent.GetRelativeTransform` (`self.SpawnPoint4`)))))

(fn `MoveTornadoLocation`
  (params (Alpha :type "Float (double-precision)"))
  (bind _returnvalue (`KismetMathLibrary.RandomFloatInRange` 250.0 500.0))
  (bind _spawnpoint_moving (`self.SpawnPoint_Moving`))
  (bind (_relativelocation_x _relativelocation_y) (`KismetMathLibrary.BreakVector` (`SceneComponent.RelativeLocation` _spawnpoint_moving)))
  (`SceneComponent.K2_SetRelativeTransform` _spawnpoint_moving (`KismetMathLibrary.TLerp` (`KismetMathLibrary.MakeTransform` (`KismetMathLibrary.MakeVector` _relativelocation_x _relativelocation_y)) (`KismetMathLibrary.MakeTransform` (`KismetMathLibrary.MakeVector` (+ _relativelocation_x _returnvalue) (+ _relativelocation_y _returnvalue))) Alpha) false true))

(fn `SpawnBankCoins`
  (bind _coinarea (`self.CoinArea`))
  (`AddComponent|NODE_AddChildActorComponent-4` :`RelativeTransform` (`KismetMathLibrary.Conv_VectorToTransform` (`KismetMathLibrary.RandomPointInBoundingBox` (`SceneComponent.RelativeLocation` _coinarea) (`BoxComponent.BoxExtent` _coinarea)))))

(fn `SpawnGems`
  (bind _coinarea (`self.CoinArea`))
  (`AddComponent|NODE_AddChildActorComponent-2` :`RelativeTransform` (`KismetMathLibrary.Conv_VectorToTransform` (`KismetMathLibrary.RandomPointInBoundingBox` (`SceneComponent.RelativeLocation` _coinarea) (`BoxComponent.BoxExtent` _coinarea)))))

(fn `SpawnMagnet`
  (bind _coinarea (`self.CoinArea`))
  (`AddComponent|NODE_AddChildActorComponent-7` :`RelativeTransform` (`KismetMathLibrary.Conv_VectorToTransform` (`KismetMathLibrary.RandomPointInBoundingBox` (`SceneComponent.RelativeLocation` _coinarea) (`BoxComponent.BoxExtent` _coinarea)))))

(fn `SpawnSpeedBoost`
  (bind _coinarea (`self.CoinArea`))
  (`AddComponent|NODE_AddChildActorComponent-9` :`RelativeTransform` (`KismetMathLibrary.Conv_VectorToTransform` (`KismetMathLibrary.RandomPointInBoundingBox` (`SceneComponent.RelativeLocation` _coinarea) (`BoxComponent.BoxExtent` _coinarea)))))

(fn `SpawnSpinMan`
  (bind _spawnpoints (`self.SpawnPoints`))
  (bind _output (`|GetArrayItem` _spawnpoints (`KismetMathLibrary.RandomIntegerInRange` 0 (`KismetArrayLibrary.Array_LastIndex` _spawnpoints))))
  (bind _returnvalue (`AddComponent|NODE_AddSkeletalMeshComponent-0` :`RelativeTransform` (`KismetMathLibrary.MakeTransform` (.location _output) (`KismetMathLibrary.MakeRotator` (.roll (.rotation _output)) (.pitch (.rotation _output)) (+ (.yaw (.rotation _output)) 90.0)) (2.0 2.0 2.0))))
  (set `self.SpinnyMan` _returnvalue))

(fn `SpawnTornadoes`
  (bind _returnvalue (`AddComponent|NODE_AddChildActorComponent-14` :`RelativeTransform` (`SceneComponent.GetRelativeTransform` (`self.SpawnPoint_Moving`))))
  (set `self.Tornado` _returnvalue)
  (set `self.bHasTornadoSpawned?` true))

(fn `SpawnTurret`
  (bind _currenttileindex (`/Game/Blueprints/BP_GameMode.CurrentTileIndex` (`self.GameModeRef`)))
  (if (or (== _currenttileindex 10) (== _currenttileindex 20))
    (`AddComponent|NODE_AddChildActorComponent-8` :`RelativeTransform` (`KismetMathLibrary.Conv_VectorToTransform` (`SceneComponent.RelativeLocation` (`self.TurretSpawn1`))))
    (`AddComponent|NODE_AddChildActorComponent-10` :`RelativeTransform` (`KismetMathLibrary.Conv_VectorToTransform` (`SceneComponent.RelativeLocation` (`self.TurretSpawn2`))))))

(fn `SpawnWall`
  (bind _wallspawn (`self.WallSpawn`))
  (bind (_relativelocation_x _relativelocation_y _relativelocation_z) (`KismetMathLibrary.BreakVector` (`SceneComponent.RelativeLocation` _wallspawn)))
  (if (== (`/Game/Blueprints/BP_GameMode.CurrentTileIndex` (`self.GameModeRef`)) 20)
    (`AddComponent|NODE_AddChildActorComponent-11` :`RelativeTransform` (`KismetMathLibrary.MakeTransform` (`KismetMathLibrary.MakeVector` _relativelocation_x (+ _relativelocation_y (`KismetMathLibrary.RandomFloatInRange` -500.0 500.0)) _relativelocation_z) (`SceneComponent.RelativeRotation` _wallspawn)))))

(fn `UserConstructionScript`
  (`|ExecutionSequence`
    (:`then_0`
      (bind _asbp_game_mode (cast `/Game/Blueprints/BP_GameMode` (`GameplayStatics.GetGameMode`)))
      (set `self.GameModeRef` _asbp_game_mode)
      (`self.GetSpawnPoints`))
    (:`then_1`
      (`self.SpawnWall`)
      (`self.SpawnGems`))
    (:`then_2`
      (switch `int` (`KismetMathLibrary.RandomIntegerInRange` 0 5)
        (:`0`
          (`self.SpawnBankCoins`))
        (:`1`
          (`self.SpawnSpinMan`)
          (set `self.bHasSpinManSpawned?` true))
        (:`2`
          (`self.SpawnMagnet`))
        (:`3`
          (`self.SpawnTurret`))
        (:`4`
          (`self.SpawnSpeedBoost`))
        (:`5`
          (`self.SpawnTornadoes`)
          (set `self.bHasTornadoSpawned?` true))))))