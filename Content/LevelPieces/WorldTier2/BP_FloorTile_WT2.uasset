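; BP_FloorTile_WT2 is a World Tier 2 floor tile level piece that randomly decorates itself with an obstacle or prop spawned by SpawnLog.
; The construction script runs the parent's logic, then calls SpawnLog, which on a 50% chance adds a child actor component at a random point inside the CoinArea box.
; The event graph holds only disabled placeholder events.
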(fn `SpawnLog`
  (bind _coinarea (`self.CoinArea`))
  (if (`KismetMathLibrary.RandomBoolWithWeight` 0.5)
    (`AddComponent|NODE_AddChildActorComponent-0` :`RelativeTransform` (`KismetMathLibrary.Conv_VectorToTransform` (`KismetMathLibrary.RandomPointInBoundingBox` (`SceneComponent.RelativeLocation` _coinarea) (`BoxComponent.BoxExtent` _coinarea))))))

(fn `UserConstructionScript`
  (`parent.UserConstructionScript`)
  (`self.SpawnLog`))