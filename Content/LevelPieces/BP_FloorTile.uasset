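; Endless-runner floor tile that has BP_GameMode add another tile when the player reaches its EndTrigger, then destroys itself after a delay.
; The construction script adds a randomly placed obstacle and optional coins, plus walls, turrets, bank coins, magnets or speed boosts gated by CurrentTileIndex, mostly against random numbers.
; A timeline started on BeginPlay spins and moves the obstacle vertically.
; KillZone overlap plays a sound and calls GameComplete on the player.
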(event `self.EndTrigger.OnComponentBeginOverlap`
  (params (OverlappedComponent :type "PrimitiveComponent Object Reference") (OtherActor :type "Actor Object Reference") (OtherComp :type "PrimitiveComponent Object Reference") (OtherBodyIndex :type Integer) (bFromSweep :type Boolean) (SweepResult :type "HitResult Structure (by ref)"))
  (cast `/Game/Blueprints/BP_Player` OtherActor)
  (bind _asbp_game_mode (cast `/Game/Blueprints/BP_GameMode` (`GameplayStatics.GetGameMode`)))
  (`/Game/Blueprints/BP_GameMode.AddFloorTile` _asbp_game_mode)
  (`KismetSystemLibrary.Delay` 10.0)
  (`self.K2_DestroyActor`))

(event `self.ReceiveBeginPlay`
  (bind _obstacle (`self.Obstacle`))
  (bind (_direction _spin _location) (`Timeline|Timeline_0`)
    (:`Update`
      (`/Engine/EditorBlueprintResources/StandardMacros.IsValid` (`self.Obstacle`)
        (:`Is Valid`
          (`SceneComponent.K2_AddRelativeRotation` _obstacle (`KismetMathLibrary.MakeRotator` 0.0 0.0 _spin) false false)
          (`SceneComponent.K2_AddRelativeLocation` _obstacle (`KismetMathLibrary.MakeVector` 0.0 0.0 _location) false false))))))

(event `self.KillZone.OnComponentBeginOverlap`
  (params (OverlappedComponent :type "PrimitiveComponent Object Reference") (OtherActor :type "Actor Object Reference") (OtherComp :type "PrimitiveComponent Object Reference") (OtherBodyIndex :type Integer) (bFromSweep :type Boolean) (SweepResult :type "HitResult Structure (by ref)"))
  (bind _asbp_player (cast `/Game/Blueprints/BP_Player` OtherActor))
  (`GameplayStatics.PlaySoundAtLocation` "/Game/Assets/Audio/grandma_loves_ping_pong_too_much_Cue.grandma_loves_ping_pong_too_much_Cue" (`SceneComponent.K2_GetComponentLocation` (`/Game/Blueprints/BP_Player.Player` _asbp_player)) (struct) 1.0 1.0 0.0 null null null)
  (`/Game/Blueprints/BP_Player.GameComplete` _asbp_player))

(fn `GetAttachTransform`
  (returns (AttachTransform :type "Transform Structure"))
  (return (`SceneComponent.K2_GetComponentToWorld` (`self.AttachPoint`))))

(fn `GetSpawnPoints`
  (set `self.SpawnPoints` (`|MakeArray` (`SceneComponent.GetRelativeTransform` (`self.SpawnPoint5`)) (`SceneComponent.GetRelativeTransform` (`self.SpawnPoint7`)) (`SceneComponent.GetRelativeTransform` (`self.SpawnPoint3`)) (`SceneComponent.GetRelativeTransform` (`self.SpawnPoint9`)))))

(fn `SpawnBankCoins`
  (bind _coinarea (`self.CoinArea`))
  (`AddComponent|NODE_AddChildActorComponent-4` :`RelativeTransform` (`KismetMathLibrary.Conv_VectorToTransform` (`KismetMathLibrary.RandomPointInBoundingBox` (`SceneComponent.RelativeLocation` _coinarea) (`BoxComponent.BoxExtent` _coinarea)))))

(fn `SpawnCoins`
  (bind _coinarea (`self.CoinArea`))
  (`AddComponent|NODE_AddChildActorComponent-2` :`RelativeTransform` (`KismetMathLibrary.Conv_VectorToTransform` (`KismetMathLibrary.RandomPointInBoundingBox` (`SceneComponent.RelativeLocation` _coinarea) (`BoxComponent.BoxExtent` _coinarea)))))

(fn `SpawnMagnet`
  (bind _coinarea (`self.CoinArea`))
  (`AddComponent|NODE_AddChildActorComponent-7` :`RelativeTransform` (`KismetMathLibrary.Conv_VectorToTransform` (`KismetMathLibrary.RandomPointInBoundingBox` (`SceneComponent.RelativeLocation` _coinarea) (`BoxComponent.BoxExtent` _coinarea)))))

(fn `SpawnObstacles`
  (bind _spawnpoints (`self.SpawnPoints`))
  (bind _output (`|GetArrayItem` _spawnpoints (`KismetMathLibrary.RandomIntegerInRange` 0 (`KismetArrayLibrary.Array_LastIndex` _spawnpoints))))
  (bind _returnvalue (`AddComponent|NODE_AddSkeletalMeshComponent-0` :`RelativeTransform` (`KismetMathLibrary.MakeTransform` (.location _output) (`KismetMathLibrary.MakeRotator` (.roll (.rotation _output)) (.pitch (.rotation _output)) (+ (.yaw (.rotation _output)) 90.0)) (2.0 2.0 2.0))))
  (set `self.Obstacle` _returnvalue))

(fn `SpawnSpeedBoost`
  (bind _coinarea (`self.CoinArea`))
  (`AddComponent|NODE_AddChildActorComponent-9` :`RelativeTransform` (`KismetMathLibrary.Conv_VectorToTransform` (`KismetMathLibrary.RandomPointInBoundingBox` (`SceneComponent.RelativeLocation` _coinarea) (`BoxComponent.BoxExtent` _coinarea)))))

(fn `SpawnTurret`
  (`AddComponent|NODE_AddChildActorComponent-8` :`RelativeTransform` (`KismetMathLibrary.Conv_VectorToTransform` (`SceneComponent.RelativeLocation` (`self.TurretSpawn1`))))
  (`AddComponent|NODE_AddChildActorComponent-10` :`RelativeTransform` (`KismetMathLibrary.Conv_VectorToTransform` (`SceneComponent.RelativeLocation` (`self.TurretSpawn2`)))))

(fn `SpawnWall`
  (bind _wallspawn (`self.WallSpawn`))
  (bind (_relativelocation_x _relativelocation_y _relativelocation_z) (`KismetMathLibrary.BreakVector` (`SceneComponent.RelativeLocation` _wallspawn)))
  (`AddComponent|NODE_AddChildActorComponent-11` :`RelativeTransform` (`KismetMathLibrary.MakeTransform` (`KismetMathLibrary.MakeVector` _relativelocation_x (+ _relativelocation_y (`KismetMathLibrary.RandomFloatInRange` -500.0 500.0)) _relativelocation_z) (`SceneComponent.RelativeRotation` _wallspawn))))

(fn `UserConstructionScript`
  (`|ExecutionSequence`
    (:`then_0`
      (bind _asbp_game_mode (cast `/Game/Blueprints/BP_GameMode` (`GameplayStatics.GetGameMode`)))
      (if (== (`/Game/Blueprints/BP_GameMode.CurrentTileIndex` _asbp_game_mode) (`KismetMathLibrary.RandomIntegerInRange` 30 40))
        (`self.SpawnWall`)))
    (:`then_1`
      (`self.GetSpawnPoints`)
      (`self.SpawnObstacles`)
      (if (`KismetMathLibrary.RandomBool`)
        (`self.SpawnCoins`)))
    (:`then_2`
      (bind _asbp_game_mode_2 (cast `/Game/Blueprints/BP_GameMode` (`GameplayStatics.GetGameMode`)))
      (if (== (`/Game/Blueprints/BP_GameMode.CurrentTileIndex` _asbp_game_mode_2) (`KismetMathLibrary.RandomIntegerInRange` 5 25))
        (`self.SpawnBankCoins`)))
    (:`then_3`
      (bind _asbp_game_mode_3 (cast `/Game/Blueprints/BP_GameMode` (`GameplayStatics.GetGameMode`)))
      (if (== (`/Game/Blueprints/BP_GameMode.CurrentTileIndex` _asbp_game_mode_3) (`KismetMathLibrary.RandomIntegerInRange` 15 25))
        (`self.SpawnMagnet`)))
    (:`then_4`
      (bind _asbp_game_mode_4 (cast `/Game/Blueprints/BP_GameMode` (`GameplayStatics.GetGameMode`)))
      (bind _currenttileindex (`/Game/Blueprints/BP_GameMode.CurrentTileIndex` _asbp_game_mode_4))
      (if (or (== _currenttileindex 10) (== _currenttileindex 20))
        (`self.SpawnTurret`)))
    (:`then_5`
      (bind _asbp_game_mode_5 (cast `/Game/Blueprints/BP_GameMode` (`GameplayStatics.GetGameMode`)))
      (bind _currenttileindex_2 (`/Game/Blueprints/BP_GameMode.CurrentTileIndex` _asbp_game_mode_5))
      (if (or (== _currenttileindex_2 (`KismetMathLibrary.RandomIntegerInRange` 1 10)) (== (`KismetMathLibrary.RandomIntegerInRange` 10 20) _currenttileindex_2))
        (`self.SpawnSpeedBoost`)))))